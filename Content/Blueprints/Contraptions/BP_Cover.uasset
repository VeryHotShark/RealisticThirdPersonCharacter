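; Spline-based cover actor that characters snap to, slide along and leave, with red transparent instanced meshes laid along the spline in the construction script.
; Enter and exit play standing or crouch montages chosen by a sphere trace, with motion warping aligning entry to the nearest spline point.
; Position updates advance along the spline using the animation Speed curve, wrapping on loops or clamping and notifying the cover component at open ends.
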(event EventUpdateCharacterPosition
  (params (Character :type Character%20Object%20Reference) (CoverComponent :type Character%20Cover%20Component%20Object%20Reference) (MoveDirection :type Float%20%28single-precision%29))
  ;[0.3589 0.3801 1] Cover Tick
  (bind _distance (CallFunction|CalculateDesiredSplineDistance Character MoveDirection))
  (CallFunction|CheckforCoverEnd CoverComponent _distance MoveDirection)
  (Transformation|SetActorLocationAndRotation Character (.Location (CallFunction|GetClosestSplineLocationRotationatDistance Character _distance)) (.Rotation (CallFunction|GetClosestSplineLocationRotationatDistance Character _distance))))

(event EventExitCover
  (params (Character :type Character%20Object%20Reference) (CoverComponent :type Character%20Cover%20Component%20Object%20Reference))
  (bind _returnvalue (Transformation|GetActorLocation Character))
  (bind _mesh (Variables|/Script/Engine.Character|GetMesh Character))
  (bind _returnvalue_2 (CallFunction|GetClosestSplineDistanceatLocation _returnvalue))
  (bind (_location _rotation) (CallFunction|GetClosestSplineLocationRotationatDistance Character _returnvalue_2))
  ;[1 0.2789 0.2729] Handle Cover Exit. Pick Correct Montage
  (Utilities|Array|RemoveItem (Variables|Default|GetCharactersInCover) Character)
  (bind _highcover (CallFunction|CheckCoverTypeatLocation _location _rotation))
  (Animation|Montage|PlayMontage _mesh (select _highcover "/Game/Characters/Katiusza/Animations/Retargeted/AM_Cover_Exit.AM_Cover_Exit" "/Game/Characters/Katiusza/Animations/Retargeted/AM_CrouchCover_Exit.AM_CrouchCover_Exit")
    (:then
      (Class|CharacterCoverComponent|SetCoverTransitionState CoverComponent true))
    (:OnCompleted
      (Class|CharacterCoverComponent|SetCoverTransitionState CoverComponent false :!label _label)
      (Class|AnimInstance|SetRootMotionMode (Components|SkeletalMesh|GetAnimInstance _mesh) "RootMotionFromEverything"))
    (:OnBlendOut
      (goto _label))))

(event EventEnterCover
  (params (Character :type Character%20Object%20Reference) (CoverComponent :type Character%20Cover%20Component%20Object%20Reference))
  (bind _returnvalue (Transformation|GetActorLocation Character))
  (bind _mesh (Variables|/Script/Engine.Character|GetMesh Character))
  (bind _returnvalue_2 (CallFunction|GetClosestSplineDistanceatLocation _returnvalue))
  (bind (_location _rotation) (CallFunction|GetClosestSplineLocationRotationatDistance Character _returnvalue_2))
  ;[0.6271 1 0.5771] Handle Cover Enter. Calculate Position and Pick Correct Montage
  (Utilities|Array|Add (Variables|Default|GetCharactersInCover) Character)
  (Class|MotionWarpingComponent|AddorUpdateWarpTargetfromLocationandRotation (Actor|GetComponentbyClass Character "/Script/MotionWarping.MotionWarpingComponent") "WarpTarget" _location _rotation)
  (bind _highcover (CallFunction|CheckCoverTypeatLocation _location _rotation))
  (Animation|Montage|PlayMontage _mesh (select _highcover "/Game/Characters/Katiusza/Animations/Retargeted/AM_Cover_Enter.AM_Cover_Enter" "/Game/Characters/Katiusza/Animations/Retargeted/AM_CrouchCover_Enter.AM_CrouchCover_Enter")
    (:then
      (Class|CharacterCoverComponent|SetCoverTransitionState CoverComponent true))
    (:OnCompleted
      (Class|CharacterCoverComponent|SetCoverTransitionState CoverComponent false :!label _label)
      (Class|AnimInstance|SetRootMotionMode (Components|SkeletalMesh|GetAnimInstance _mesh) "IgnoreRootMotion"))
    (:OnBlendOut
      (goto _label))))

(fn ConstructionScript
  (bind _pointmesh (LocalVariables|GetPointMesh))
  (bind _spline (Variables|Default|GetSpline))
  (bind _instancedstaticmesh (Variables|Default|GetInstancedStaticMesh))
  (bind _meshoffset (LocalVariables|GetMeshOffset))
  (bind _returnvalue (StaticMesh|GetBoundingBox _pointmesh))
  (bind (_min _max) (Utilities|Struct|BreakBox _returnvalue))
  (bind _returnvalue_2 (- _max _min))
  (bind _returnvalue_3 (+ (.x _returnvalue_2) _meshoffset))
  (Spline|SetClosedLoop (Variables|Default|GetSpline) (Variables|Default|GetLoopCover) true)
  (Components|InstancedStaticMesh|ClearInstances (Variables|Default|GetInstancedStaticMesh))
  (Components|StaticMesh|SetStaticMesh _instancedstaticmesh (LocalVariables|GetPointMesh))
  (Rendering|Material|SetMaterial _instancedstaticmesh 0 "/Game/StarterContent/Materials/MI_Transparent_Red.MI_Transparent_Red")
  (for _index (range 0 (Math|Float|Floor (/ (Spline|GetSplineLength (Variables|Default|GetSpline)) _returnvalue_3)))
    (Components|InstancedStaticMesh|AddInstance (Variables|Default|GetInstancedStaticMesh) (Math|Transform|MakeTransform (Spline|GetLocationatDistanceAlongSpline _spline (* _index _returnvalue_3) "Local") (Spline|GetRotationatDistanceAlongSpline _spline (* _index _returnvalue_3) "Local")) false)))

(fn GetClosestSplineDistanceatLocation
  (params (Location :type Vector :default "0, 0, 0"))
  (bind _spline (Variables|Default|GetSpline))
  (return (Class|SplineComponent|GetDistanceAlongSplineatSplineInputKey _spline (Class|SplineComponent|FindInputKeyClosesttoWorldLocation _spline Location))))

(fn GetClosestSplineLocationRotationatDistance
  (params (Character :type Character%20Object%20Reference) (Distance :type Float%20%28single-precision%29))
  (bind _spline (Variables|Default|GetSpline))
  (return (+ (Math|Vector|MakeVector 0.0 0.0 (Components|Capsule|GetScaledCapsuleHalfHeight (Variables|/Script/Engine.Character|GetCapsuleComponent Character))) (Spline|GetLocationatDistanceAlongSpline _spline Distance "World")) (Math|Rotator|Delta(Rotator) (Spline|GetRotationatDistanceAlongSpline _spline Distance "Local") "0.000000,-90.000000,0.000000")))

(fn CalculateDesiredSplineDistance
  (params (Character :type Character%20Object%20Reference) (MoveDirection :type Float%20%28double-precision%29))
  (bind _returnvalue (Utilities|Time|GetWorldDeltaSeconds))
  (bind _returnvalue_2 (Transformation|GetActorLocation Character))
  (bind _mesh (Variables|/Script/Engine.Character|GetMesh Character))
  (bind _movecoverspeed (Variables|Default|GetMoveCoverSpeed))
  (bind _spline (Variables|Default|GetSpline))
  (bind _returnvalue_3 (Components|SkeletalMesh|GetAnimInstance _mesh))
  (bind _returnvalue_4 (Spline|GetSplineLength _spline))
  (bind _returnvalue_5 (CallFunction|GetClosestSplineDistanceatLocation _returnvalue_2))
  (bind _outvalue (Class|AnimInstance|GetCurveValuewithDefault _returnvalue_3 "Speed" _movecoverspeed))
  (bind _returnvalue_6 (* _returnvalue _outvalue MoveDirection))
  (bind _returnvalue_7 (+ _returnvalue_5 _returnvalue_6))
  (if (Class|SplineComponent|IsClosedLoop (Variables|Default|GetSpline))
    (return (Class|KismetMathLibrary|FWrap _returnvalue_7 0.0 _returnvalue_4))
    (else
      (return (Math|Float|Clamp(Float) _returnvalue_7 0.0 _returnvalue_4)))))

(fn CheckforCoverEnd
  (params (CoverComponent :type Character%20Cover%20Component%20Object%20Reference) (SplineDistance :type Float%20%28double-precision%29) (MoveDirection :type Float%20%28double-precision%29))
  (if (not (Class|SplineComponent|IsClosedLoop (Variables|Default|GetSpline)))
    (if (or (and (== SplineDistance 0.0) (< MoveDirection 0.0)) (and (> MoveDirection 0.0) (== SplineDistance (Spline|GetSplineLength (Variables|Default|GetSpline)))))
      (Class|CharacterCoverComponent|OnCoverEndReached CoverComponent MoveDirection))))

(fn CheckCoverTypeatLocation
  (params (Location :type Vector) (Rotation :type Rotator))
  (bind _returnvalue (+ Location "0.000000,0.000000,80.000000"))
  (bind _returnvalue_2 (Collision|SphereTraceForObjects _returnvalue (- _returnvalue (* (Math|Vector|GetForwardVector Rotation) 1e+02)) 2e+01 (Utilities|Array|MakeArray "ObjectTypeQuery1") false 0 "None" true "(R=1.000000,G=0.000000,B=0.000000,A=1.000000)" "(R=0.000000,G=1.000000,B=0.000000,A=1.000000)" 1.0))
  (return _returnvalue_2))