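; Animation modifier that prepares turn-in-place animations by baking curves into the sequence when applied.
; It adds a TurnInPlace metadata curve keyed to 1, then a RotationYaw curve keyed on every frame.
; Each RotationYaw key is the root bone's yaw, read with root motion extraction, remapped from zero through final-frame yaw into a clamped 0 to 1 turn progress.
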(event EventOnApply
  (params (AnimationSequence :type Anim%20Sequence%20Object%20Reference))
  (bind _output_get (Variables|Default|SetAnimation%20Sequence AnimationSequence))
  (Utilities|FlowControl|Sequence
    (:then_0
      (Class|AnimationBlueprintLibrary|AddCurve (Variables|Default|GetAnimation%20Sequence) "TurnInPlace" "RCT_Float" true)
      (Class|AnimationBlueprintLibrary|AddFloatCurveKey (Variables|Default|GetAnimation%20Sequence) "TurnInPlace" 0.0 1.0))
    (:then_1
      (Class|AnimationBlueprintLibrary|AddCurve _output_get "RotationYaw" "RCT_Float" false)
      (for _index (range 0 (Class|AnimationBlueprintLibrary|GetNumFrames (Variables|Default|GetAnimation%20Sequence)))
        (Class|AnimationBlueprintLibrary|AddFloatCurveKey (Variables|Default|GetAnimation%20Sequence) "RotationYaw" (Class|AnimationBlueprintLibrary|GetTimeatFrame (Variables|Default|GetAnimation%20Sequence) _index) (Math|Float|MapRangeClamped (.yaw (.rotation (Class|AnimationBlueprintLibrary|GetBonePoseforFrame (Variables|Default|GetAnimation%20Sequence) "root" _index true))) 0.0 (.yaw (.rotation (Class|AnimationBlueprintLibrary|GetBonePoseforFrame (Variables|Default|GetAnimation%20Sequence) "root" (Class|AnimationBlueprintLibrary|GetNumFrames (Variables|Default|GetAnimation%20Sequence)) true))) 0.0 1.0))))))