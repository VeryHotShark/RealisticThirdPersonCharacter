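; An animation modifier that bakes root motion speed into a "Speed" float curve on an animation sequence.
; On apply, it adds the curve and keys each frame from 1 onward with the Root bone's displacement since the previous frame divided by the time between them.
; The speed is the full 3D vector length, with root motion extracted, and frame 0 gets no key.
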(event EventOnApply
  (params (AnimationSequence :type Anim%20Sequence%20Object%20Reference))
  (bind _output_get (Variables|Default|SetAnimation%20Sequence AnimationSequence))
  (Class|AnimationBlueprintLibrary|AddCurve _output_get "Speed" "RCT_Float" false)
  (for _index (range 1 (Class|AnimationBlueprintLibrary|GetNumFrames (Variables|Default|GetAnimation%20Sequence)))
    (Class|AnimationBlueprintLibrary|AddFloatCurveKey (Variables|Default|GetAnimation%20Sequence) "Speed" (Class|AnimationBlueprintLibrary|GetTimeatFrame (Variables|Default|GetAnimation%20Sequence) _index) (/ (Math|Vector|VectorLength (- (.location (Class|AnimationBlueprintLibrary|GetBonePoseforFrame (Variables|Default|GetAnimation%20Sequence) "Root" _index true)) (.location (Class|AnimationBlueprintLibrary|GetBonePoseforFrame (Variables|Default|GetAnimation%20Sequence) "Root" (- _index 1) true)))) (- (Class|AnimationBlueprintLibrary|GetTimeatFrame (Variables|Default|GetAnimation%20Sequence) _index) (Class|AnimationBlueprintLibrary|GetTimeatFrame (Variables|Default|GetAnimation%20Sequence) (- _index 1)))))))