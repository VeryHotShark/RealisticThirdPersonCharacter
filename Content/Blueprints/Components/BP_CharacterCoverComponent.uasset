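; Character cover component that finds nearby cover and tracks the character's look and move direction while in cover.
; FindClosestCover runs a 200-unit sphere overlap around the character, draws a color-coded debug sphere, and returns the first Cover found rather than the nearest, with best-pick selection left as a TODO.
; UpdateCover stores move direction and passes it to the parent implementation; reaching a cover end sets look direction and zeroes movement.
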(event EventOnCoverEndReached
  (params (Direction :type Float%20%28single-precision%29))
  (Variables|Default|SetCoverLookDirection Direction)
  (Variables|Default|SetCoverMoveDirection 0.0))

(event EventUpdateCover
  (params (MoveDirection :type Float%20%28single-precision%29))
  (bind _output_get (Variables|Default|SetCoverMoveDirection MoveDirection))
  (|CallParentFunction _output_get))

(fn FindClosestCover
  (bind _character (Variables|Default|GetCharacter))
  (bind _returnvalue (Transformation|GetActorLocation _character))
  (bind (_outactors _returnvalue_2) (Collision|SphereOverlapActors _returnvalue 2e+02 (Utilities|Array|MakeArray "ObjectTypeQuery7") "/Script/RealisticMovement.Cover"))
  (Rendering|Debug|DrawDebugSphere _returnvalue 2e+02 12 (Math|Color|SelectColor "(R=0.480630,G=1.000000,B=0.266051,A=1.000000)" "(R=1.000000,G=0.113864,B=0.074062,A=1.000000)" _returnvalue_2) 0.5)
  ;[1 1 1] TODO: Choose the best one
  (for _array_element _outactors
    (bind _ascover (Utilities|Casting|CastToCover _array_element))
    (return _ascover)))